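; BP_TestCharacter is a test NPC Blueprint that opens the WBP_BurnTheVillageDialogue screen when interacted with.
; ShowInteract and HideInteract toggle its Widget component as the interaction indicator, with ShowInteract passing InRange straight into the hidden flag, so true hides it.
; InitiateInteraction creates the dialogue widget and adds it to the viewport only while that indicator is visible.
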(event `/Game/TopDown/Blueprints/BPI_Interact.Show Interact`
  (params (InRange :type Boolean))
  (`SceneComponent.SetHiddenInGame` (`self.Widget`) InRange false))

(event `/Game/TopDown/Blueprints/BPI_Interact.Hide Interact`
  (`SceneComponent.SetHiddenInGame` (`self.Widget`) true false))

(event `/Game/TopDown/Blueprints/BPI_Interact.Initiate Interaction`
  (if (`WidgetComponent.IsWidgetVisible` (`self.Widget`))
    (bind _returnvalue (`|CreateWidget` "/Game/OurFuckingFolder/UI/WBP_BurnTheVillageDialogue.WBP_BurnTheVillageDialogue_C"))
    (`UserWidget.AddToViewport` _returnvalue 0)))

(fn `UserConstructionScript`)